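; Flipper actor, likely pinball-style, that swings back and forth automatically on a timed loop with no player input.
; The construction script uses FlipType to set mirrored start and end rotations, apply the starting pose, and flip the mesh's X scale for the right-hand variant.
; BeginPlay alternates the Flip and Flop events with one-second delays, each using MoveComponentTo to rotate the Flipper component over FlipTime.
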(event Custom|Flip
  (Components|MoveComponentTo (Variables|Default|GetFlipper) "0, 0, 0" (Variables|Default|GetEndRotation) false false (Variables|Default|GetFlipTime) false))

(event Custom|Flop
  (Components|MoveComponentTo (Variables|Default|GetFlipper) "0, 0, 0" (Variables|Default|GetStartRotation) false false (Variables|Default|GetFlipTime) false))

(event EventBeginPlay
  (Utilities|FlowControl|Delay 1.0 :!label _label)
  (CallFunction|Flip)
  (Utilities|FlowControl|Delay 1.0)
  (CallFunction|Flop)
  (goto _label))

(event Collision|EventActorBeginOverlap
  (params (OtherActor :type Actor%20Object%20Reference)))

(event EventTick
  (params (DeltaSeconds :type Float%20%28single-precision%29)))

(fn ConstructionScript
  (Variables|Default|SetStartRotation (Utilities|Select :Index (Variables|Default|GetFlipType) :NewEnumerator0 "0,20.000000, 0" :NewEnumerator1 "0,-20.000000, 0"))
  (Variables|Default|SetEndRotation (Utilities|Select :Index (Variables|Default|GetFlipType) :NewEnumerator0 "0,-20.000000, 0" :NewEnumerator1 "0,20.000000, 0"))
  (Transformation|SetRelativeRotation (Variables|Default|GetFlipper) (Variables|Default|GetStartRotation) false false)
  (switch Utilities|FlowControl|Switch|SwitchonFlipperEnum (Variables|Default|GetFlipType)
    (:NewEnumerator1
      (Transformation|SetRelativeScale3D (Variables|Default|GetFlipper) "-1.000000,1.000000,1.000000"))))