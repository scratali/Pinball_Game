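; BP_Slingshot is a pinball slingshot that kicks the ball away and awards points when hit.
; On overlap with a BP_Ball, it adds score through PinballGameMode and applies a velocity-change impulse opposite the Capsule's forward vector.
; It then restarts a timeline that drives the PercentOut parameter on a dynamic material instance, created in the construction script, to animate the hit through the material.
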(event EventBeginPlay)

(event Collision|EventActorBeginOverlap
  (params (OtherActor :type Actor%20Object%20Reference))
  (bind _asbp_ball (Utilities|Casting|CastToBP_Ball OtherActor))
  (bind _aspinball_game_mode (Utilities|Casting|CastToPinballGameMode (Game|GetGameMode))
    (:then
      (Default|AddScore _aspinball_game_mode 2e+01))
    (:CastFailed
      _))
  (Physics|AddImpulse (Variables|/Game/Blueprints/BP_Ball.BP_Ball_C|GetBall _asbp_ball) (* (* (Math|Vector|GetForwardVector (Variables|Default|GetCapsule)) -1.0) 2.5e+03) "None" true)
  (bind _percent (Timeline|MorphT_TimeLine PlayFromStart)
    (:Update
      (Rendering|Material|SetScalarParameterValue (Variables|Default|GetMorphTMaterialIns) "PercentOut" _percent :!class /Script/Engine.MaterialInstanceDynamic))))

(fn ConstructionScript
  (bind _returnvalue (Rendering|Material|CreateDynamicMaterialInstance (Variables|Default|GetStaticMesh) 2 0 "None" :!class /Script/Engine.PrimitiveComponent))
  (Variables|Default|SetMorphTMaterialIns _returnvalue))