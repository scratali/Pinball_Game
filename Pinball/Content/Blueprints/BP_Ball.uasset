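; BP_Ball is a ball actor that is pushed continuously and kept against the table surface beneath it.
; Each Tick applies a frame-time-scaled DefaultSpeed impulse to the Ball component as a velocity change, ignoring mass.
; It then line-traces down from the actor and, on a hit, adds an impulse along the inverted impact normal, scaled by TableStickiness, to press the ball onto the surface.
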(event EventBeginPlay)

(event Collision|EventActorBeginOverlap
  (params (OtherActor :type Actor%20Object%20Reference)))

(event EventTick
  (params (DeltaSeconds :type Float%20%28single-precision%29))
  (bind _returnvalue (Transformation|GetActorLocation))
  (Physics|AddImpulse (Variables|Default|GetBall) (* (Variables|Default|GetDefaultSpeed) DeltaSeconds) "None" true)
  (bind (_outhit _returnvalue_2) (Collision|LineTraceByChannel _returnvalue (- _returnvalue "0,0.000000,500.000000") "TraceTypeQuery1" false 0 "None"))
  (if _returnvalue_2
    (Physics|AddImpulse (Variables|Default|GetBall) (* (* (.ImpactNormal (Collision|BreakHitResult _outhit)) -1.0) (* (Variables|Default|GetTableStickiness) DeltaSeconds)) "None" true)))

(fn ConstructionScript)