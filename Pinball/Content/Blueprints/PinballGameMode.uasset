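; Game mode for a pinball game that runs the main menu, ball lives, multiplied scoring and menu music.
; ResetGame restores class defaults, and each ball spawned at the plunger respawns through its OnDestroyed binding until none remain.
; Game over opens high score entry if the score qualifies against a lazily loaded, cached save, otherwise the main menu.
; Music starts with the menu, and StopMusic fades it out on a timeline.
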(event Custom|SpawnBall
  (bind _outactors (Actor|GetAllActorsOfClass "/Game/Blueprints/BP_Plunger.BP_Plunger_C"))
  (bind _returnvalue (Game|SpawnActorfromClass "/Game/Blueprints/BP_Ball.BP_Ball_C" (Math|Conversions|ToTransform(Vector) (Default|GetBallSpawnLocation (Utilities|Array|Get(acopy) _outactors))) "Undefined" 0 0))
  (Game|BindEventtoOnDestroyed _returnvalue (delegate Custom|BallDestroyed)))

(event Custom|BallDestroyed
  (params (DestroyedActor :type Actor%20Object%20Reference))
  (bind _result (Math|Integer|DecrementInt (Variables|Default|GetBallsRemaining))
    (:%20%20
      (if (> _result 0)
        (CallFunction|SpawnBall)
        (else
          (CallFunction|EndGame))))))

(event Custom|EndGame
  (bind _currentsaveobject (CallFunction|GetSaveGameData))
  (if (<= (Utilities|Array|Length (Variables|/Game/Blueprints/HighScoreSave.HighScoreSave_C|GetSaveStruct _currentsaveobject)) 3)
    (CallFunction|CreateHighScoreList :!label _label)
    (else
      (bind _lowestscorestruct (Default|DetermineLowestScoreValue _currentsaveobject))
      (if (< (.score _lowestscorestruct) (Variables|Default|GetScore))
        (goto _label)
        (else
          (CallFunction|CreateMainMenu))))))

(event Custom|CreateHighScoreList
  (bind _returnvalue (Game|GetPlayerController 0))
  (bind _aspinball_player_controller (Utilities|Casting|CastToPinball_PlayerController _returnvalue))
  (bind _returnvalue_2 (UserInterface|CreateWidget "/Game/Blueprints/HighScoreEntry.HighScoreEntry_C" _aspinball_player_controller))
  (UserInterface|Viewport|AddtoViewport _returnvalue_2 0)
  (Variables|/Script/Engine.PlayerController|SetbShowMouseCursor _aspinball_player_controller true))

(event Custom|CreateMainMenu
  (bind _returnvalue (Game|GetPlayerController 0))
  (bind _aspinball_player_controller (Utilities|Casting|CastToPinball_PlayerController _returnvalue))
  (CallFunction|GetSaveGameData)
  (Viewport|RemoveAllWidgets)
  (bind _returnvalue_2 (UserInterface|CreateWidget "/Game/Blueprints/MainMenu.MainMenu_C" _aspinball_player_controller))
  (UserInterface|Viewport|AddtoViewport _returnvalue_2 0)
  (Variables|/Script/Engine.PlayerController|SetbShowMouseCursor _aspinball_player_controller true)
  (CallFunction|StartMusic))

(event Custom|ResetGame
  (bind _returnvalue (Game|GetPlayerController 0))
  (bind (_score _multiplier _ballsremaining) (Utilities|GetClassDefaults "PinballGameMode_C"))
  (bind _aspinball_player_controller (Utilities|Casting|CastToPinball_PlayerController _returnvalue))
  (Variables|Default|SetScore _score)
  (Variables|Default|SetMultiplier _multiplier)
  (Variables|Default|SetBallsRemaining _ballsremaining)
  (CallFunction|SpawnBall)
  (Default|CreatePlayerHUD _aspinball_player_controller)
  (Variables|/Script/Engine.PlayerController|SetbShowMouseCursor _aspinball_player_controller false)
  (Default|CallOnGameReset))

(event Custom|StopMusic
  (bind _volume (Timeline|StopMusicTimeLine PlayFromStart)
    (:Update
      (Audio|Components|Audio|SetVolumeMultiplier (Variables|Default|GetMainMusic) (Math|Float|Lerp 0.0 0.2 _volume) :!class /Script/Engine.AudioComponent))
    (:Finished
      (Audio|Components|Audio|Stop (Variables|Default|GetMainMusic)))))

(event Custom|StartMusic
  (bind _mainmusic (Variables|Default|GetMainMusic)
    (:then
      _)
    (:else
      (CallFunction|SpawnMusic)))
  (if (not (Audio|Components|Audio|IsPlaying _mainmusic))
    (Audio|Components|Audio|Play (Variables|Default|GetMainMusic) 0.0)))

(event Custom|SpawnMusic
  (bind _returnvalue (Audio|SpawnSound2D "/Game/Assets/Sounds/victoryMusic_loop_Cue.victoryMusic_loop_Cue" 0.25 1.0 0.0 0))
  (Variables|Default|SetMainMusic _returnvalue))

(event EventBeginPlay
  (CallFunction|CreateMainMenu))

(event EventTick
  (params (DeltaSeconds :type Float%20%28single-precision%29)))

(fn ConstructionScript)

(fn AddScore
  (params (PointsToAdd :type Float%20%28single-precision%29))
  (bind _output_get (Variables|Default|SetScore (+ (* PointsToAdd (Variables|Default|GetMultiplier)) (Variables|Default|GetScore))))
  (return _output_get))

(fn GetSaveGameData
  (bind _currentsaveobject (Variables|Default|GetCurrentSaveObject)
    (:then
      (return _currentsaveobject))
    (:else
      (bind _returnvalue (SaveGame|DoesSaveGameExist (Variables|Default|GetHighScoreSaveName)))
      (if _returnvalue
        (bind _returnvalue_2 (SaveGame|LoadGamefromSlot (Variables|Default|GetHighScoreSaveName)))
        (bind _ashigh_score_save (Utilities|Casting|CastToHighScoreSave _returnvalue_2))
        (Default|SortSaveData _ashigh_score_save)
        (bind _output_get (Variables|Default|SetCurrentSaveObject _ashigh_score_save))
        (return _output_get)
        (else
          (bind _returnvalue_3 (SaveGame|CreateSaveGameObject "/Game/Blueprints/HighScoreSave.HighScoreSave_C"))
          (bind _output_get_2 (Variables|Default|SetCurrentSaveObject _returnvalue_3))
          (return _output_get_2))))))